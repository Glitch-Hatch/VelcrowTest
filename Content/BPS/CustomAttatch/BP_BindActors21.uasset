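; Snappable cube actor that binds to other BP_BindActors21 cubes when their HitBox-tagged components overlap.
; Four Binder and Binded overlap events record component pairs, then move them into both actors' ConnectedComponents maps.
; The first unconnected pair triggers SnapRotation, which uses dot products to align nearest axes, then offsets CubeMesh and joins both meshes with a fully locked runtime physics constraint.
; Tick keeps the actor transform on CubeMesh and prints its location.
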(event OnComponentBeginOverlap(Binder1)
  (params (OverlappedComponent :type Primitive%20Component%20Object%20Reference) (OtherActor :type Actor%20Object%20Reference) (OtherComp :type Primitive%20Component%20Object%20Reference) (OtherBodyIndex :type Integer) (bFromSweep :type Boolean) (SweepResult :type Hit%20Result%20Structure%20%28by%20ref%29))
  (CallFunction|BoxOverlapWhileHolding OverlappedComponent OtherComp)
  (bind (_keypin _valuepin) (Utilities|Map|ForEachLoop(Map) (Variables|Default|GetOverlappedComponents))
    (:then
      (if (not (and (Utilities|Map|Contains (Variables|Default|GetConnectedComponents) _keypin) (.bSuccess (Utilities|Casting|CastToBP_BindActors21 (Components|GetOwner _valuepin)))))
        (if (not (Utilities|Map|Contains (Variables|BP_BindActors21_C|GetConnectedComponents (.AsBP%20Bind%20Actors%2021 (Utilities|Casting|CastToBP_BindActors21 (Components|GetOwner _valuepin)))) _valuepin))
          (Utilities|FlowControl|Sequence
            (:then_0
              (Utilities|FlowControl|DoOnce false :!label _label
                (:Completed
                  (Utilities|FlowControl|Sequence
                    (:then_0
                      (Variables|Default|SetConnectedParent (.AsBP%20Bind%20Actors%2021 (Utilities|Casting|CastToBP_BindActors21 (Components|GetOwner _valuepin))))
                      (CallFunction|SnapRotation (.AsBP%20Bind%20Actors%2021 (Utilities|Casting|CastToBP_BindActors21 (Components|GetOwner _valuepin)))))
                    (:then_1
                      (Transformation|SetWorldLocation (Variables|Default|GetCubeMesh) (+ (Transformation|GetWorldLocation (Variables|Default|GetCubeMesh)) (- (Transformation|GetWorldLocation _valuepin) (Transformation|GetWorldLocation _keypin))) false true)
                      (bind _returnvalue (AddComponent|AddPhysicsConstraintComponent true (Math|Transform|MakeTransform (Transformation|GetWorldLocation _keypin) (Transformation|GetWorldRotation _keypin) "1.000000,1.000000,1.000000")))
                      (Variables|Default|SetConstraint _returnvalue)
                      (Class|PhysicsConstraintComponent|SetConstrainedComponents (Variables|Default|GetConstraint) (Variables|Default|GetCubeMesh) "None" (Variables|BP_BindActors21_C|GetCubeMesh (.AsBP%20Bind%20Actors%2021 (Utilities|Casting|CastToBP_BindActors21 (Components|GetOwner _valuepin)))) "None")
                      (Class|PhysicsConstraintComponent|SetLinearXLimit (Variables|Default|GetConstraint) "LCM_Locked" 0.0)
                      (Class|PhysicsConstraintComponent|SetLinearYLimit (Variables|Default|GetConstraint) "LCM_Locked" 0.0)
                      (Class|PhysicsConstraintComponent|SetLinearZLimit (Variables|Default|GetConstraint) "LCM_Locked" 0.0)
                      (Class|PhysicsConstraintComponent|SetAngularSwing1Limit (Variables|Default|GetConstraint) "ACM_Locked" 0.0)
                      (Class|PhysicsConstraintComponent|SetAngularSwing2Limit (Variables|Default|GetConstraint) "ACM_Locked" 0.0)
                      (Class|PhysicsConstraintComponent|SetAngularTwistLimit (Variables|Default|GetConstraint) "ACM_Locked" 0.0))))))
            (:then_1
              (Utilities|Map|Add (Variables|Default|GetConnectedComponents) _keypin _valuepin)
              (Utilities|Map|Remove (Variables|Default|GetOverlappedComponents) _keypin)
              (Utilities|Map|Remove (Variables|BP_BindActors21_C|GetOverlappedComponents (.AsBP%20Bind%20Actors%2021 (Utilities|Casting|CastToBP_BindActors21 (Components|GetOwner _valuepin)))) _valuepin)
              (Utilities|Map|Add (Variables|BP_BindActors21_C|GetConnectedComponents (.AsBP%20Bind%20Actors%2021 (Utilities|Casting|CastToBP_BindActors21 (Components|GetOwner _valuepin)))) _valuepin _keypin))))))
    (:CompletedPin
      (goto _label Reset))))

(event OnComponentBeginOverlap(Binded1)
  (params (OverlappedComponent :type Primitive%20Component%20Object%20Reference) (OtherActor :type Actor%20Object%20Reference) (OtherComp :type Primitive%20Component%20Object%20Reference) (OtherBodyIndex :type Integer) (bFromSweep :type Boolean) (SweepResult :type Hit%20Result%20Structure%20%28by%20ref%29))
  (CallFunction|BoxOverlapWhileHolding OverlappedComponent OtherComp)
  (bind (_keypin _valuepin) (Utilities|Map|ForEachLoop(Map) (Variables|Default|GetOverlappedComponents))
    (:then
      (if (not (and (Utilities|Map|Contains (Variables|Default|GetConnectedComponents) _keypin) (.bSuccess (Utilities|Casting|CastToBP_BindActors21 (Components|GetOwner _valuepin)))))
        (if (not (Utilities|Map|Contains (Variables|BP_BindActors21_C|GetConnectedComponents (.AsBP%20Bind%20Actors%2021 (Utilities|Casting|CastToBP_BindActors21 (Components|GetOwner _valuepin)))) _valuepin))
          (Utilities|FlowControl|Sequence
            (:then_0
              (Utilities|FlowControl|DoOnce false :!label _label
                (:Completed
                  (Utilities|FlowControl|Sequence
                    (:then_0
                      (Variables|Default|SetConnectedParent (.AsBP%20Bind%20Actors%2021 (Utilities|Casting|CastToBP_BindActors21 (Components|GetOwner _valuepin))))
                      (CallFunction|SnapRotation (.AsBP%20Bind%20Actors%2021 (Utilities|Casting|CastToBP_BindActors21 (Components|GetOwner _valuepin)))))
                    (:then_1
                      (Transformation|SetWorldLocation (Variables|Default|GetCubeMesh) (+ (Transformation|GetWorldLocation (Variables|Default|GetCubeMesh)) (- (Transformation|GetWorldLocation _valuepin) (Transformation|GetWorldLocation _keypin))) false true)
                      (bind _returnvalue (AddComponent|AddPhysicsConstraintComponent true (Math|Transform|MakeTransform (Transformation|GetWorldLocation _keypin) (Transformation|GetWorldRotation _keypin) "1.000000,1.000000,1.000000")))
                      (Variables|Default|SetConstraint _returnvalue)
                      (Class|PhysicsConstraintComponent|SetConstrainedComponents (Variables|Default|GetConstraint) (Variables|Default|GetCubeMesh) "None" (Variables|BP_BindActors21_C|GetCubeMesh (.AsBP%20Bind%20Actors%2021 (Utilities|Casting|CastToBP_BindActors21 (Components|GetOwner _valuepin)))) "None")
                      (Class|PhysicsConstraintComponent|SetLinearXLimit (Variables|Default|GetConstraint) "LCM_Locked" 0.0)
                      (Class|PhysicsConstraintComponent|SetLinearYLimit (Variables|Default|GetConstraint) "LCM_Locked" 0.0)
                      (Class|PhysicsConstraintComponent|SetLinearZLimit (Variables|Default|GetConstraint) "LCM_Locked" 0.0)
                      (Class|PhysicsConstraintComponent|SetAngularSwing1Limit (Variables|Default|GetConstraint) "ACM_Locked" 0.0)
                      (Class|PhysicsConstraintComponent|SetAngularSwing2Limit (Variables|Default|GetConstraint) "ACM_Locked" 0.0)
                      (Class|PhysicsConstraintComponent|SetAngularTwistLimit (Variables|Default|GetConstraint) "ACM_Locked" 0.0))))))
            (:then_1
              (Utilities|Map|Add (Variables|Default|GetConnectedComponents) _keypin _valuepin)
              (Utilities|Map|Remove (Variables|Default|GetOverlappedComponents) _keypin)
              (Utilities|Map|Remove (Variables|BP_BindActors21_C|GetOverlappedComponents (.AsBP%20Bind%20Actors%2021 (Utilities|Casting|CastToBP_BindActors21 (Components|GetOwner _valuepin)))) _valuepin)
              (Utilities|Map|Add (Variables|BP_BindActors21_C|GetConnectedComponents (.AsBP%20Bind%20Actors%2021 (Utilities|Casting|CastToBP_BindActors21 (Components|GetOwner _valuepin)))) _valuepin _keypin))))))
    (:CompletedPin
      (goto _label Reset))))

(event OnComponentBeginOverlap(Binder2)
  (params (OverlappedComponent :type Primitive%20Component%20Object%20Reference) (OtherActor :type Actor%20Object%20Reference) (OtherComp :type Primitive%20Component%20Object%20Reference) (OtherBodyIndex :type Integer) (bFromSweep :type Boolean) (SweepResult :type Hit%20Result%20Structure%20%28by%20ref%29))
  (CallFunction|BoxOverlapWhileHolding OverlappedComponent OtherComp)
  (bind (_keypin _valuepin) (Utilities|Map|ForEachLoop(Map) (Variables|Default|GetOverlappedComponents))
    (:then
      (if (not (and (Utilities|Map|Contains (Variables|Default|GetConnectedComponents) _keypin) (.bSuccess (Utilities|Casting|CastToBP_BindActors21 (Components|GetOwner _valuepin)))))
        (if (not (Utilities|Map|Contains (Variables|BP_BindActors21_C|GetConnectedComponents (.AsBP%20Bind%20Actors%2021 (Utilities|Casting|CastToBP_BindActors21 (Components|GetOwner _valuepin)))) _valuepin))
          (Utilities|FlowControl|Sequence
            (:then_0
              (Utilities|FlowControl|DoOnce false :!label _label
                (:Completed
                  (Utilities|FlowControl|Sequence
                    (:then_0
                      (Variables|Default|SetConnectedParent (.AsBP%20Bind%20Actors%2021 (Utilities|Casting|CastToBP_BindActors21 (Components|GetOwner _valuepin))))
                      (CallFunction|SnapRotation (.AsBP%20Bind%20Actors%2021 (Utilities|Casting|CastToBP_BindActors21 (Components|GetOwner _valuepin)))))
                    (:then_1
                      (Transformation|SetWorldLocation (Variables|Default|GetCubeMesh) (+ (Transformation|GetWorldLocation (Variables|Default|GetCubeMesh)) (- (Transformation|GetWorldLocation _valuepin) (Transformation|GetWorldLocation _keypin))) false true)
                      (bind _returnvalue (AddComponent|AddPhysicsConstraintComponent true (Math|Transform|MakeTransform (Transformation|GetWorldLocation _keypin) (Transformation|GetWorldRotation _keypin) "1.000000,1.000000,1.000000")))
                      (Variables|Default|SetConstraint _returnvalue)
                      (Class|PhysicsConstraintComponent|SetConstrainedComponents (Variables|Default|GetConstraint) (Variables|Default|GetCubeMesh) "None" (Variables|BP_BindActors21_C|GetCubeMesh (.AsBP%20Bind%20Actors%2021 (Utilities|Casting|CastToBP_BindActors21 (Components|GetOwner _valuepin)))) "None")
                      (Class|PhysicsConstraintComponent|SetLinearXLimit (Variables|Default|GetConstraint) "LCM_Locked" 0.0)
                      (Class|PhysicsConstraintComponent|SetLinearYLimit (Variables|Default|GetConstraint) "LCM_Locked" 0.0)
                      (Class|PhysicsConstraintComponent|SetLinearZLimit (Variables|Default|GetConstraint) "LCM_Locked" 0.0)
                      (Class|PhysicsConstraintComponent|SetAngularSwing1Limit (Variables|Default|GetConstraint) "ACM_Locked" 0.0)
                      (Class|PhysicsConstraintComponent|SetAngularSwing2Limit (Variables|Default|GetConstraint) "ACM_Locked" 0.0)
                      (Class|PhysicsConstraintComponent|SetAngularTwistLimit (Variables|Default|GetConstraint) "ACM_Locked" 0.0))))))
            (:then_1
              (Utilities|Map|Add (Variables|Default|GetConnectedComponents) _keypin _valuepin)
              (Utilities|Map|Remove (Variables|Default|GetOverlappedComponents) _keypin)
              (Utilities|Map|Remove (Variables|BP_BindActors21_C|GetOverlappedComponents (.AsBP%20Bind%20Actors%2021 (Utilities|Casting|CastToBP_BindActors21 (Components|GetOwner _valuepin)))) _valuepin)
              (Utilities|Map|Add (Variables|BP_BindActors21_C|GetConnectedComponents (.AsBP%20Bind%20Actors%2021 (Utilities|Casting|CastToBP_BindActors21 (Components|GetOwner _valuepin)))) _valuepin _keypin))))))
    (:CompletedPin
      (goto _label Reset))))

(event OnComponentBeginOverlap(Binded2)
  (params (OverlappedComponent :type Primitive%20Component%20Object%20Reference) (OtherActor :type Actor%20Object%20Reference) (OtherComp :type Primitive%20Component%20Object%20Reference) (OtherBodyIndex :type Integer) (bFromSweep :type Boolean) (SweepResult :type Hit%20Result%20Structure%20%28by%20ref%29))
  (CallFunction|BoxOverlapWhileHolding OverlappedComponent OtherComp)
  (bind (_keypin _valuepin) (Utilities|Map|ForEachLoop(Map) (Variables|Default|GetOverlappedComponents))
    (:then
      (if (not (and (Utilities|Map|Contains (Variables|Default|GetConnectedComponents) _keypin) (.bSuccess (Utilities|Casting|CastToBP_BindActors21 (Components|GetOwner _valuepin)))))
        (if (not (Utilities|Map|Contains (Variables|BP_BindActors21_C|GetConnectedComponents (.AsBP%20Bind%20Actors%2021 (Utilities|Casting|CastToBP_BindActors21 (Components|GetOwner _valuepin)))) _valuepin))
          (Utilities|FlowControl|Sequence
            (:then_0
              (Utilities|FlowControl|DoOnce false :!label _label
                (:Completed
                  (Utilities|FlowControl|Sequence
                    (:then_0
                      (Variables|Default|SetConnectedParent (.AsBP%20Bind%20Actors%2021 (Utilities|Casting|CastToBP_BindActors21 (Components|GetOwner _valuepin))))
                      (CallFunction|SnapRotation (.AsBP%20Bind%20Actors%2021 (Utilities|Casting|CastToBP_BindActors21 (Components|GetOwner _valuepin)))))
                    (:then_1
                      (Transformation|SetWorldLocation (Variables|Default|GetCubeMesh) (+ (Transformation|GetWorldLocation (Variables|Default|GetCubeMesh)) (- (Transformation|GetWorldLocation _valuepin) (Transformation|GetWorldLocation _keypin))) false true)
                      (bind _returnvalue (AddComponent|AddPhysicsConstraintComponent true (Math|Transform|MakeTransform (Transformation|GetWorldLocation _keypin) (Transformation|GetWorldRotation _keypin) "1.000000,1.000000,1.000000")))
                      (Variables|Default|SetConstraint _returnvalue)
                      (Class|PhysicsConstraintComponent|SetConstrainedComponents (Variables|Default|GetConstraint) (Variables|Default|GetCubeMesh) "None" (Variables|BP_BindActors21_C|GetCubeMesh (.AsBP%20Bind%20Actors%2021 (Utilities|Casting|CastToBP_BindActors21 (Components|GetOwner _valuepin)))) "None")
                      (Class|PhysicsConstraintComponent|SetLinearXLimit (Variables|Default|GetConstraint) "LCM_Locked" 0.0)
                      (Class|PhysicsConstraintComponent|SetLinearYLimit (Variables|Default|GetConstraint) "LCM_Locked" 0.0)
                      (Class|PhysicsConstraintComponent|SetLinearZLimit (Variables|Default|GetConstraint) "LCM_Locked" 0.0)
                      (Class|PhysicsConstraintComponent|SetAngularSwing1Limit (Variables|Default|GetConstraint) "ACM_Locked" 0.0)
                      (Class|PhysicsConstraintComponent|SetAngularSwing2Limit (Variables|Default|GetConstraint) "ACM_Locked" 0.0)
                      (Class|PhysicsConstraintComponent|SetAngularTwistLimit (Variables|Default|GetConstraint) "ACM_Locked" 0.0))))))
            (:then_1
              (Utilities|Map|Add (Variables|Default|GetConnectedComponents) _keypin _valuepin)
              (Utilities|Map|Remove (Variables|Default|GetOverlappedComponents) _keypin)
              (Utilities|Map|Remove (Variables|BP_BindActors21_C|GetOverlappedComponents (.AsBP%20Bind%20Actors%2021 (Utilities|Casting|CastToBP_BindActors21 (Components|GetOwner _valuepin)))) _valuepin)
              (Utilities|Map|Add (Variables|BP_BindActors21_C|GetConnectedComponents (.AsBP%20Bind%20Actors%2021 (Utilities|Casting|CastToBP_BindActors21 (Components|GetOwner _valuepin)))) _valuepin _keypin))))))
    (:CompletedPin
      (goto _label Reset))))

(event Custom|HelloThisIsMyTestEVent
  (params (OverlappedComponent :type Primitive%20Component%20Object%20Reference) (OtherActor :type Actor%20Object%20Reference) (OtherComp :type Primitive%20Component%20Object%20Reference) (OtherBodyIndex :type Integer) (bFromSweep :type Boolean) (SweepResult :type Hit%20Result%20Structure%20%28by%20ref%29)))

(event EventTick
  (params (DeltaSeconds :type Float%20%28single-precision%29))
  (bind _returnvalue (Transformation|GetActorTransform))
  (bind _cubemesh (Variables|Default|GetCubeMesh))
  (bind (_location _rotation) (Math|Transform|BreakTransform _returnvalue))
  (bind _returnvalue_2 (Transformation|GetWorldLocation _cubemesh))
  (Transformation|SetActorLocationAndRotation _returnvalue_2 (Transformation|GetWorldRotation _cubemesh) false true)
  (Transformation|SetWorldLocationAndRotation (Variables|Default|GetCubeMesh) _location _rotation false false)
  (Development|PrintString (Utilities|String|ToString(Vector) _returnvalue_2)))

(fn ConstructionScript)

(fn BoxOverlapWhileHolding
  (params (Overlapped%20Comp :type Primitive%20Component%20Object%20Reference) (Other%20Comp :type Primitive%20Component%20Object%20Reference))
  (bind _returnvalue (Components|GetOwner Other%20Comp))
  (bind (_asbp_bind_actors_21 _bsuccess) (Utilities|Casting|CastToBP_BindActors21 _returnvalue))
  (if (Math|Boolean|ANDBoolean (Utilities|Array|ContainsItem (Variables|/Script/Engine.ActorComponent|GetComponentTags Other%20Comp) "HitBox") _bsuccess (!= Other%20Comp self))
    (if (not (Utilities|Map|Contains (Variables|BP_BindActors21_C|GetConnectedComponents _asbp_bind_actors_21) Other%20Comp))
      (Utilities|Map|Add (Variables|Default|GetOverlappedComponents) Overlapped%20Comp Other%20Comp))))

(fn SnapRotation
  (params (self2 :type BP%20Bind%20Actors%2021%20Object%20Reference))
  (bind _cubemesh (Variables|Default|GetCubeMesh))
  (bind _cubemesh_2 (Variables|BP_BindActors21_C|GetCubeMesh self2))
  (bind _cubemesh_3 (Variables|Default|GetCubeMesh))
  (bind _cubemesh_4 (Variables|Default|GetCubeMesh))
  (bind _returnvalue (Math|Vector|GetUpVector _cubemesh_2))
  (bind _returnvalue_2 (Math|Vector|GetRightVector _cubemesh_2))
  (bind _returnvalue_3 (Math|Vector|GetForwardVector _cubemesh_3))
  (bind _returnvalue_4 (Math|Vector|GetUpVector _cubemesh_3))
  (bind _returnvalue_5 (Math|Vector|GetRightVector _cubemesh_3))
  (bind _returnvalue_6 (Math|Vector|GetUpVector _cubemesh_4))
  (bind _returnvalue_7 (Math|Vector|GetRightVector _cubemesh_4))
  (bind _returnvalue_8 (Math|Vector|GetForwardVector _cubemesh_2))
  (bind _returnvalue_9 (Math|Vector|GetForwardVector _cubemesh))
  (bind _returnvalue_10 (Math|Vector|GetUpVector _cubemesh))
  (bind _returnvalue_11 (Math|Vector|GetRightVector _cubemesh))
  (bind _returnvalue_12 (Math|Vector|DotProduct _returnvalue_8 _returnvalue_3))
  (bind _returnvalue_13 (Math|Vector|DotProduct _returnvalue_8 _returnvalue_4))
  (bind _returnvalue_14 (Math|Vector|DotProduct _returnvalue_8 _returnvalue_5))
  (bind _returnvalue_15 (Math|Vector|DotProduct _returnvalue _returnvalue))
  (bind _returnvalue_16 (Math|Vector|DotProduct _returnvalue _returnvalue))
  (bind _returnvalue_17 (Math|Vector|DotProduct _returnvalue _returnvalue))
  (bind _returnvalue_18 (Math|Vector|DotProduct _returnvalue_9 _returnvalue_2))
  (bind _returnvalue_19 (Math|Vector|DotProduct _returnvalue_10 _returnvalue_2))
  (bind _returnvalue_20 (Math|Vector|DotProduct _returnvalue_11 _returnvalue_2))
  (bind _returnvalue_21 (Math|Float|Absolute(Float) _returnvalue_12))
  (bind _returnvalue_22 (Math|Float|Absolute(Float) _returnvalue_13))
  (bind _returnvalue_23 (Math|Float|Absolute(Float) _returnvalue_14))
  (bind _returnvalue_24 (Math|Float|Absolute(Float) _returnvalue_15))
  (bind _returnvalue_25 (Math|Float|Absolute(Float) _returnvalue_16))
  (bind _returnvalue_26 (Math|Float|Absolute(Float) _returnvalue_17))
  (bind _returnvalue_27 (Math|Float|Absolute(Float) _returnvalue_18))
  (bind _returnvalue_28 (Math|Float|Absolute(Float) _returnvalue_19))
  (bind _returnvalue_29 (Math|Float|Absolute(Float) _returnvalue_20))
  (bind _returnvalue_30 (Math|Float|Max(Float) _returnvalue_27 _returnvalue_28 _returnvalue_29))
  (bind _returnvalue_31 (Math|Float|Max(Float) _returnvalue_21 _returnvalue_22 _returnvalue_23))
  (bind _returnvalue_32 (Math|Float|Max(Float) _returnvalue_24 _returnvalue_25 _returnvalue_26))
  (Utilities|FlowControl|Sequence
    (:then_0
      (if (== _returnvalue_21 _returnvalue_31)
        (Transformation|AddWorldRotation (Variables|Default|GetCubeMesh) (Class|KismetMathLibrary|QuatRotator (Class|KismetMathLibrary|QuatFindBetweenVectors (select (> _returnvalue_12 0.0) _returnvalue_3 (* _returnvalue_3 -1.0)) _returnvalue_8)) false false)
        (elif (== _returnvalue_22 _returnvalue_31)
          (Transformation|AddWorldRotation (Variables|Default|GetCubeMesh) (Class|KismetMathLibrary|QuatRotator (Class|KismetMathLibrary|QuatFindBetweenVectors (select (> _returnvalue_13 0.0) _returnvalue_4 (* _returnvalue_4 -1.0)) _returnvalue_8)) false false)
          (elif (== _returnvalue_23 _returnvalue_31)
            (Transformation|AddWorldRotation (Variables|Default|GetCubeMesh) (Class|KismetMathLibrary|QuatRotator (Class|KismetMathLibrary|QuatFindBetweenVectors (select (> _returnvalue_14 0.0) _returnvalue_5 (* _returnvalue_5 -1.0)) _returnvalue_8)) false false)))))
    (:then_1
      (if (== _returnvalue_24 _returnvalue_32)
        (Transformation|AddWorldRotation (Variables|Default|GetCubeMesh) (Class|KismetMathLibrary|QuatRotator (Class|KismetMathLibrary|QuatFindBetweenVectors (select (> _returnvalue_15 0.0) "0, 0, 0" (* (Math|Vector|GetForwardVector _cubemesh_4) -1.0)) _returnvalue)) false false)
        (elif (== _returnvalue_25 _returnvalue_32)
          (Transformation|AddWorldRotation (Variables|Default|GetCubeMesh) (Class|KismetMathLibrary|QuatRotator (Class|KismetMathLibrary|QuatFindBetweenVectors (select (> _returnvalue_16 0.0) _returnvalue_6 (* _returnvalue_6 -1.0)) _returnvalue)) false false)
          (elif (== _returnvalue_26 _returnvalue_32)
            (Transformation|AddWorldRotation (Variables|Default|GetCubeMesh) (Class|KismetMathLibrary|QuatRotator (Class|KismetMathLibrary|QuatFindBetweenVectors (select (> _returnvalue_17 0.0) _returnvalue_7 (* _returnvalue_7 -1.0)) _returnvalue)) false false)))))
    (:then_2
      (if (== _returnvalue_27 _returnvalue_30)
        (Transformation|AddWorldRotation (Variables|Default|GetCubeMesh) (Class|KismetMathLibrary|QuatRotator (Class|KismetMathLibrary|QuatFindBetweenVectors (select (> _returnvalue_18 0.0) "0, 0, 0" (* _returnvalue_9 -1.0)) _returnvalue_2)) false false)
        (elif (== _returnvalue_28 _returnvalue_30)
          (Transformation|AddWorldRotation (Variables|Default|GetCubeMesh) (Class|KismetMathLibrary|QuatRotator (Class|KismetMathLibrary|QuatFindBetweenVectors (select (> _returnvalue_19 0.0) _returnvalue_10 (* _returnvalue_10 -1.0)) _returnvalue_2)) false false)
          (elif (== _returnvalue_29 _returnvalue_30)
            (Transformation|AddWorldRotation (Variables|Default|GetCubeMesh) (Class|KismetMathLibrary|QuatRotator (Class|KismetMathLibrary|QuatFindBetweenVectors (select (> _returnvalue_20 0.0) _returnvalue_11 (* _returnvalue_11 -1.0)) _returnvalue_2)) false false)))))))