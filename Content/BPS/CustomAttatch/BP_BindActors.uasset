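; BP_BindActors is a cube actor that snaps and binds to other cubes of its kind through two bind components.
; When either overlaps a "Binder"-tagged component, it positions the other cube beyond that side, matches its rotation and attaches its own cube to it.
; Tick sweeps the cube to its current location every frame.
; BeginPlay caches a BP_BindParent that goes unused, and the delayed unbind logic is unwired.
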(event OnComponentBeginOverlap(Binded1)
  (params (OverlappedComponent :type Primitive%20Component%20Object%20Reference) (OtherActor :type Actor%20Object%20Reference) (OtherComp :type Primitive%20Component%20Object%20Reference) (OtherBodyIndex :type Integer) (bFromSweep :type Boolean) (SweepResult :type Hit%20Result%20Structure%20%28by%20ref%29))
  (Variables|Default|SetOther%20Comp OtherComp)
  (Variables|Default|SetOverlapped%20Component OverlappedComponent)
  (if (Utilities|Array|ContainsItem (Variables|/Script/Engine.ActorComponent|GetComponentTags (Variables|Default|GetOther%20Comp)) "Binder")
    (Transformation|SetWorldLocation (Variables|BP_BindActors_C|GetCubeMesh (.AsBP%20Bind%20Actors (Utilities|Casting|CastToBP_BindActors (Components|GetOwner (Variables|Default|GetOther%20Comp))))) (+ (Transformation|GetWorldLocation (Variables|Default|GetCubeMesh)) (* (+ (- (Transformation|GetWorldLocation (Variables|Default|GetOverlapped%20Component)) (Transformation|GetWorldLocation (Variables|Default|GetCubeMesh))) (* (Math|Vector|Normalize (- (Transformation|GetWorldLocation (Variables|Default|GetOverlapped%20Component)) (Transformation|GetWorldLocation (Variables|Default|GetCubeMesh)))) 12.5)) 2.0)) false false)
    (Transformation|SetWorldRotation (Variables|BP_BindActors_C|GetCubeMesh (.AsBP%20Bind%20Actors (Utilities|Casting|CastToBP_BindActors (Components|GetOwner (Variables|Default|GetOther%20Comp))))) (Transformation|GetWorldRotation (Variables|Default|GetCubeMesh)) false false)
    (Transformation|AttachComponentToComponent (Variables|Default|GetCubeMesh) (Variables|BP_BindActors_C|GetCubeMesh (.AsBP%20Bind%20Actors (Utilities|Casting|CastToBP_BindActors (Components|GetOwner (Variables|Default|GetOther%20Comp))))) "None" "KeepWorld" "KeepWorld" "KeepWorld" true)))

(event OnComponentBeginOverlap(Binded2)
  (params (OverlappedComponent :type Primitive%20Component%20Object%20Reference) (OtherActor :type Actor%20Object%20Reference) (OtherComp :type Primitive%20Component%20Object%20Reference) (OtherBodyIndex :type Integer) (bFromSweep :type Boolean) (SweepResult :type Hit%20Result%20Structure%20%28by%20ref%29))
  (Variables|Default|SetOther%20Comp OtherComp)
  (Variables|Default|SetOverlapped%20Component OverlappedComponent)
  (if (Utilities|Array|ContainsItem (Variables|/Script/Engine.ActorComponent|GetComponentTags (Variables|Default|GetOther%20Comp)) "Binder")
    (Transformation|SetWorldLocation (Variables|BP_BindActors_C|GetCubeMesh (.AsBP%20Bind%20Actors (Utilities|Casting|CastToBP_BindActors (Components|GetOwner (Variables|Default|GetOther%20Comp))))) (+ (Transformation|GetWorldLocation (Variables|Default|GetCubeMesh)) (* (+ (- (Transformation|GetWorldLocation (Variables|Default|GetOverlapped%20Component)) (Transformation|GetWorldLocation (Variables|Default|GetCubeMesh))) (* (Math|Vector|Normalize (- (Transformation|GetWorldLocation (Variables|Default|GetOverlapped%20Component)) (Transformation|GetWorldLocation (Variables|Default|GetCubeMesh)))) 12.5)) 2.0)) false false)
    (Transformation|SetWorldRotation (Variables|BP_BindActors_C|GetCubeMesh (.AsBP%20Bind%20Actors (Utilities|Casting|CastToBP_BindActors (Components|GetOwner (Variables|Default|GetOther%20Comp))))) (Transformation|GetWorldRotation (Variables|Default|GetCubeMesh)) false false)
    (Transformation|AttachComponentToComponent (Variables|Default|GetCubeMesh) (Variables|BP_BindActors_C|GetCubeMesh (.AsBP%20Bind%20Actors (Utilities|Casting|CastToBP_BindActors (Components|GetOwner (Variables|Default|GetOther%20Comp))))) "None" "KeepWorld" "KeepWorld" "KeepWorld" true)))

(event EventBeginPlay
  (bind _outactors (Actor|GetAllActorsOfClass "/Game/BPS/CustomAttatch/BP_BindParent.BP_BindParent_C"))
  (bind _array_element (Utilities|Array|ForEachLoopwithBreak _outactors :!label _label)
    (:LoopBody
      (Variables|Default|SetBindParent _array_element)
      (goto _label Break))))

(event Collision|EventActorBeginOverlap
  (params (OtherActor :type Actor%20Object%20Reference)))

(event EventTick
  (params (DeltaSeconds :type Float%20%28single-precision%29))
  (Transformation|SetWorldLocation (Variables|Default|GetCubeMesh) (Transformation|GetWorldLocation (Variables|Default|GetCubeMesh)) true false))

(fn ConstructionScript)